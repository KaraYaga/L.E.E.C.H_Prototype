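; Base game manager that evaluates the player's stats for emails and game-over conditions.
; It caches GI_BASE on BeginPlay; the comments note that the Game Instance calls GM_StatCheck.
; That check passes the instance to BossEmailsREF for email sending, then compares Morale and CompanyPerformance against DataAsset minimums.
; Each failed check independently shows its Die or Fired game-over widget and enables the mouse cursor.
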(event `self.ReceiveBeginPlay`
  ;[0.09375 0.2992 1] Reference Game Instance
  (bind _asgi_base (cast `/Game/_GameManager/GI_BASE` (`GameplayStatics.GetGameInstance`)))
  (set `self.GameInstance` _asgi_base))

(event `GM_StatCheck`
  (bind _dataasset (`self.DataAsset`))
  (bind _gameinstance (`self.GameInstance`))
  ;[1 0.01173 0.5473] Check Stats (After called by Game Instance) GAME OVER CONDITIONS
  ;;[1 0.2611 0.8716] Check Stats Compare to Emails (Receive Email if ==)
  (`/Game/_Widgets/Emails/WBP_BossEmails.SendEmail` (`self.BossEmails_REF`) (`self.GameInstance`))
  (`|ExecutionSequence`
    (:`then_0`
      (if (<= (`/Game/_GameManager/GI_BASE.Morale` _gameinstance) (`/Game/DataAssets_Base/StatusDataAsset.MIN Morale` _dataasset))
        (bind _returnvalue (`|CreateWidget` "/Game/_Widgets/GameOvers/WBP_GameOver_Die.WBP_GameOver_Die_C"))
        (`UserWidget.AddToViewport` _returnvalue 0)
        (set `PlayerController.bShowMouseCursor` true (`GameplayStatics.GetPlayerController` 0))))
    (:`then_1`
      (if (<= (`/Game/_GameManager/GI_BASE.CompanyPerformance` _gameinstance) (`/Game/DataAssets_Base/StatusDataAsset.MIN Company Progress` _dataasset))
        (bind _returnvalue_2 (`|CreateWidget` "/Game/_Widgets/GameOvers/WBP_GameOver_Fired.WBP_GameOver_Fired_C"))
        (`UserWidget.AddToViewport` _returnvalue_2 0)
        (set `PlayerController.bShowMouseCursor` true (`GameplayStatics.GetPlayerController` 0))))))

(fn `UserConstructionScript`)